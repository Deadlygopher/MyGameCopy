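; BP_Item_World_Actor is the in-world representation of an inventory item.
; On BeginPlay it copies the mesh and scale from its Item class defaults onto ItemMesh, and passes the item name and Amount to the WB_Item widget in ItemWB.
; Interact_Collision overlap events cast to BP_Player_Character but take no further action.
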(event OnComponentBeginOverlap(Interact_Collision)
  (params (OverlappedComponent :type Primitive%20Component%20Object%20Reference) (OtherActor :type Actor%20Object%20Reference) (OtherComp :type Primitive%20Component%20Object%20Reference) (OtherBodyIndex :type Integer) (bFromSweep :type Boolean) (SweepResult :type Hit%20Result%20Structure%20%28by%20ref%29))
  (Utilities|Casting|CastToBP_Player_Character OtherActor))

(event OnComponentEndOverlap(Interact_Collision)
  (params (OverlappedComponent :type Primitive%20Component%20Object%20Reference) (OtherActor :type Actor%20Object%20Reference) (OtherComp :type Primitive%20Component%20Object%20Reference) (OtherBodyIndex :type Integer))
  (Utilities|Casting|CastToBP_Player_Character OtherActor))

(event EventBeginPlay
  (CallFunction|SetItemMesh)
  (CallFunction|SetItemName))

(fn ConstructionScript)

(fn SetItemMesh
  (bind _item_mesh (Variables|Default|GetItem%20Mesh))
  (bind _item (Variables|Default|GetItem))
  (bind _itemstructure (Utilities|GetClassDefaults _item))
  (Components|StaticMesh|SetStaticMesh _item_mesh (.itemmesh _itemstructure))
  (Transformation|SetWorldScale3D _item_mesh (.meshscale _itemstructure)))

(fn SetItemName
  (bind _aswb_item (Utilities|Casting|CastToWB_Item (UserInterface|GetUserWidgetObject (Variables|Default|GetItem%20WB))))
  (Default|SetNameandAmount _aswb_item (.itemname (Utilities|GetClassDefaults (Variables|Default|GetItem))) (Variables|Default|GetAmount)))