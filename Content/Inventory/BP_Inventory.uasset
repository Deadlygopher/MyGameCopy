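; BP_Inventory is a slot-based inventory that stores item classes with amounts and creates its own hidden WB_Inventory widget on the player interface canvas.
; The slot array is sized at BeginPlay, and item properties such as stack limits come from class defaults.
; AddItem tops up matching stacks, looping on overflow, then puts any remainder into the first empty slot, returning a result enum.
; RefreshSlotInfo updates individual slot widgets separately from AddItem.
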(event EventBeginPlay
  (Utilities|Array|Resize (Variables|Default|GetSlot%20Array) (Variables|Default|GetAmount%20of%20Slot)))

(fn ConstructionScript)

(fn GetSlotData
  (params (Index :type Integer))
  (bind _slot_array (Variables|Default|GetSlot%20Array))
  (bind _output (Utilities|Array|Get(acopy) _slot_array Index))
  (if (Utilities|IsValidClass (.item _output))
    (return false (Utilities|GetClassDefaults (.item _output)) (.amount _output))
    (else
      (return true "" 0))))

(fn CreateInventoryWidget
  (bind _returnvalue (UserInterface|CreateWidget "/Game/Inventory/Widget/WB_Inventory.WB_Inventory_C" 0 self))
  (bind _output_get (Variables|Default|SetInventory_WB_Ref _returnvalue))
  (bind _returnvalue_2 (Class|CanvasPanel|AddChildtoCanvas (Variables|/Game/UI/WB_PlayerInterface.WB_PlayerInterface_C|GetPlayerCanvasPanel (Variables|Default|GetPlayerInterface_WB_Ref)) _output_get))
  (Class|CanvasPanelSlot|SetAutoSize _returnvalue_2 true)
  (Class|CanvasPanelSlot|SetPosition _returnvalue_2 "(X=700.000000,Y=540.000000)")
  (Widget|SetVisibility (Variables|Default|GetInventory_WB_Ref) "Hidden"))

(fn RefreshSlotInfo
  (params (Slot%20Index :type Integer))
  (Default|UpdateItemInfo (Utilities|Array|Get(acopy) (Variables|/Game/Inventory/Widget/WB_Inventory.WB_Inventory_C|GetSlot_WB (Variables|Default|GetInventory_WB_Ref)) Slot%20Index)))

(fn FindEmptySlot
  (bind (_array_element _array_index) (Utilities|Array|ForEachLoopwithBreak (Variables|Default|GetSlot%20Array) :!label _label)
    (:LoopBody
      (if (not (Utilities|IsValidClass (.Item (Utilities|Struct|BreakSlotStructure _array_element))))
        (LocalVariables|SetSlotFound true)
        (goto _label Break)))
    (:Completed
      (return _array_index (LocalVariables|GetSlotFound)))))

(fn FindSlotforStack
  (params (Item :type BP%20Master%20Item%20Class%20Reference))
  (bind (_array_element _array_index) (Utilities|Array|ForEachLoopwithBreak (Variables|Default|GetSlot%20Array) :!label _label)
    (:LoopBody
      (if (Math|Boolean|ANDBoolean (Utilities|IsValidClass (.Item (Utilities|Struct|BreakSlotStructure _array_element))) (== (.Item (Utilities|Struct|BreakSlotStructure _array_element)) Item) (< (.Amount (Utilities|Struct|BreakSlotStructure _array_element)) (.stackamount (Utilities|GetClassDefaults (.Item (Utilities|Struct|BreakSlotStructure _array_element))))))
        (LocalVariables|SetStackFound true)
        (goto _label Break)))
    (:Completed
      (return _array_index (LocalVariables|GetStackFound)))))

(fn AddItem
  (params (Added%20Item :type BP%20Master%20Item%20Class%20Reference) (Item%20Amount :type Integer))
  (bind _slot_array (Variables|Default|GetSlot%20Array))
  (LocalVariables|SetAdded%20Item%20Local Added%20Item)
  (bind _output_get (LocalVariables|SetItem%20Amount%20Local Item%20Amount))
  (if (> _output_get 0) :!label _label
    (if (.stackable (Utilities|GetClassDefaults (LocalVariables|GetAdded%20Item%20Local)))
      (bind (_stack_slot_index _success) (CallFunction|FindSlotforStack (LocalVariables|GetAdded%20Item%20Local)))
      (if _success
        (if (<= (+ (.amount (Utilities|Array|Get(acopy) _slot_array _stack_slot_index)) (LocalVariables|GetItem%20Amount%20Local)) (.stackamount (Utilities|GetClassDefaults (.item (Utilities|Array|Get(acopy) _slot_array _stack_slot_index)))))
          (Utilities|Array|SetArrayElem _slot_array _stack_slot_index (Utilities|Struct|MakeSlotStructure (LocalVariables|GetAdded%20Item%20Local) (+ (.amount (Utilities|Array|Get(acopy) _slot_array _stack_slot_index)) (LocalVariables|GetItem%20Amount%20Local))))
          (return true "NewEnumerator1")
          (else
            (Utilities|Array|SetArrayElem (Variables|Default|GetSlot%20Array) _stack_slot_index (Utilities|Struct|MakeSlotStructure (LocalVariables|GetAdded%20Item%20Local) (.stackamount (Utilities|GetClassDefaults (.item (Utilities|Array|Get(acopy) _slot_array _stack_slot_index))))))
            (LocalVariables|SetItem%20Amount%20Local (- (LocalVariables|GetItem%20Amount%20Local) (- (.stackamount (Utilities|GetClassDefaults (.item (Utilities|Array|Get(acopy) _slot_array _stack_slot_index)))) (.amount (Utilities|Array|Get(acopy) _slot_array _stack_slot_index)))))
            (goto _label)))
        (else
          _)))
    (bind (_empty_slot_index _success_2) (CallFunction|FindEmptySlot))
    (if _success_2
      (Utilities|Array|SetArrayElem (Variables|Default|GetSlot%20Array) _empty_slot_index (Utilities|Struct|MakeSlotStructure (LocalVariables|GetAdded%20Item%20Local) (LocalVariables|GetItem%20Amount%20Local)))
      (return true "NewEnumerator0")
      (else
        (return false "NewEnumerator2")))))