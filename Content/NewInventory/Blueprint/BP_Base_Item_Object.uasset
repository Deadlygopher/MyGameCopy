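; BP_Base_Item_Object is the base data object for an inventory item, holding its class, info, icon, dimensions, stack state, amount and weight.
; Accessor functions expose this data, with setters for amount and weight.
; Rotation is a toggled flag that makes GetItemDimensions return X and Y swapped, leaving the stored dimensions untouched.
; UseItem takes a player and is an empty stub, alongside an IsUsable flag.
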(fn GetItemDimensions
  (bind _dimensions (Variables|Default|GetDimensions))
  (if (Variables|Default|GetIs%20Rotate%20?)
    (return (Utilities|Struct|MakeIntPoint (.y _dimensions) (.x _dimensions)))
    (else
      (return (Variables|Default|GetDimensions)))))

(fn GetItemClass
  (return (Variables|Default|GetItemClass)))

(fn GetItemInfo
  (return (Variables|Default|GetItem%20Info)))

(fn RotateIcon
  (Variables|Default|SetIs%20Rotate%20? (not (Variables|Default|GetIs%20Rotate%20?))))

(fn IsRotateIcon?
  (return (Variables|Default|GetIs%20Rotate%20?)))

(fn GetItemIcon
  (return (Variables|Default|GetIcon)))

(fn GetIsStack?
  (return (Variables|Default|GetIs%20Stack)))

(fn GetWeight
  (return (Variables|Default|GetWeight)))

(fn SetAmount
  (params (Amount :type Integer))
  (Variables|Default|SetAmount Amount)
  (return))

(fn GetAmount
  (return (Variables|Default|GetAmount)))

(fn GetMaxAmount
  (return (Variables|Default|GetMax%20Amount)))

(fn SetWeight
  (params (Weight :type Float%20%28single-precision%29))
  (Variables|Default|SetWeight Weight)
  (return))

(fn UseItem
  (params (Player :type BP%20New%20Inventory%20Char%20Object%20Reference)))

(fn GetIsUsable
  (return (Variables|Default|GetIs%20Usable%20?)))