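; Base world actor for a pickup item in the inventory system, collected when interacted with.
; On BeginPlay it builds a BP_Base_Item_Object from its size, icon, info and own class, unless an ItemObject is already valid.
; Interact offers that object to the given InventoryComponent and, if the add succeeds, calls ServerDestroyItem to destroy the actor.
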(event Custom|Server%20Destroy%20Item
  (Actor|DestroyActor))

(event EventBeginPlay
  (if (not (Utilities|IsValid (Variables|Default|GetItem%20Object)))
    (bind _itemobject (Private|GetDefaultItemObject))
    (Variables|Default|SetItem%20Object _itemobject)))

(event EventInteract
  (params (InventoryComponent :type BPC%20Inventory%20Object%20Reference))
  (bind _success (Default|TryAddItem InventoryComponent (Variables|Default|GetItem%20Object)))
  (if _success
    (CallFunction|ServerDestroyItem)))

(fn ConstructionScript)

(fn GetDefaultItemObject
  (bind _item_size (Variables|Default|GetItem%20Size))
  (bind _returnvalue (Game|ConstructObjectfromClass "/Game/NewInventory/Blueprint/BP_Base_Item_Object.BP_Base_Item_Object_C" self (Utilities|Struct|MakeIntPoint (Math|Float|Truncate (.x _item_size)) (Math|Float|Truncate (.y _item_size))) (Variables|Default|GetIcon) (Utilities|GetClass self) (Variables|Default|GetItem%20Info)))
  (return _returnvalue))