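; BP_Pickup_Usable_Item is an inventory pickup for usable items that carry a health-to-add value.
; GetDefaultItemObject constructs a BP_Usable_Item_Object from the pickup's properties, including grid size, icon, item info, stacking, weight and usability.
; It stores the pickup's own class on that object as ItemClass.
; The event graph holds only disabled placeholders, and construction defers to the parent.
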(event EventBeginPlay)

(event Collision|EventActorBeginOverlap
  (params (OtherActor :type Actor%20Object%20Reference)))

(event EventTick
  (params (DeltaSeconds :type Float%20%28single-precision%29)))

(fn ConstructionScript
  (|CallParentFunction))

(fn GetDefaultItemObject
  (bind _item_size (Variables|Default|GetItem%20Size))
  (bind _returnvalue (Game|ConstructObjectfromClass "/Game/NewInventory/Blueprint/BP_Usable_Item_Object.BP_Usable_Item_Object_C" self (Variables|Default|GetHealth%20to%20Add) (Utilities|Struct|MakeIntPoint (Math|Float|Truncate (.x _item_size)) (Math|Float|Truncate (.y _item_size))) (Variables|Default|GetIcon) (Utilities|GetClass self) (Variables|Default|GetItem%20Info) (Variables|Default|GetAmount) (Variables|Default|GetIs%20Stack) (Variables|Default|GetWeight) (Variables|Default|GetMax%20Amount) (Variables|Default|GetIs%20Usable%20?) 0))
  (return _returnvalue))