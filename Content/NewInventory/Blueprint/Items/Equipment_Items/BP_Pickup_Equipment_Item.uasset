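; Pickup actor for equipment items in the inventory system, carrying the item data for a piece of gear.
; On BeginPlay it creates its equipment item object unless a valid one is already set.
; GetDefaultItemObject and GetEquipmentDefaultObject contain identical logic, constructing a BP_Equipment_Item_Object owned by the actor.
; That object receives the pickup's equipment, display and stacking properties, plus the actor's own class as ItemClass.
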(event EventBeginPlay
  (|CallParentFunction)
  (if (not (Utilities|IsValid (Variables|Default|GetEquipment%20Item%20Object)))
    (bind _returnvalue (CallFunction|GetEquipmentDefaultObject))
    (Variables|Default|SetEquipment%20Item%20Object _returnvalue)))

(event Collision|EventActorBeginOverlap
  (params (OtherActor :type Actor%20Object%20Reference)))

(event EventTick
  (params (DeltaSeconds :type Float%20%28single-precision%29)))

(fn ConstructionScript
  (|CallParentFunction))

(fn GetDefaultItemObject
  (bind _returnvalue (Game|ConstructObjectfromClass "/Game/NewInventory/Blueprint/BP_Equipment_Item_Object.BP_Equipment_Item_Object_C" self (Variables|Default|GetEquipment%20Type) (Variables|Default|GetArmor%20Skeletal%20Mesh) (Variables|Default|GetProtection) (Class|KismetMathLibrary|ToIntPoint(Vector2D) (Variables|Default|GetItem%20Size)) (Variables|Default|GetIcon) (Utilities|GetClass self) (Variables|Default|GetItem%20Info) (Variables|Default|GetAmount) (Variables|Default|GetIs%20Stack) (Variables|Default|GetWeight) (Variables|Default|GetMax%20Amount) (Variables|Default|GetIs%20Usable%20?) (Variables|Default|GetWeapon%20Class)))
  (return _returnvalue))

(fn GetEquipmentDefaultObject
  (bind _returnvalue (Game|ConstructObjectfromClass "/Game/NewInventory/Blueprint/BP_Equipment_Item_Object.BP_Equipment_Item_Object_C" self (Variables|Default|GetEquipment%20Type) (Variables|Default|GetArmor%20Skeletal%20Mesh) (Variables|Default|GetProtection) (Class|KismetMathLibrary|ToIntPoint(Vector2D) (Variables|Default|GetItem%20Size)) (Variables|Default|GetIcon) (Utilities|GetClass self) (Variables|Default|GetItem%20Info) (Variables|Default|GetAmount) (Variables|Default|GetIs%20Stack) (Variables|Default|GetWeight) (Variables|Default|GetMax%20Amount) (Variables|Default|GetIs%20Usable%20?) (Variables|Default|GetWeapon%20Class)))
  (return _returnvalue))