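; Player inventory component that stores items in a tile grid (Column x Row) and toggles the inventory widget.
; Multi-tile items occupy every covered index in a flat array; adding tries stacking, then free space, then retries with the item rotated.
; Split stacks seek an empty slot, falling back to a world drop.
; Dropping spawns the item actor ahead of the player via a ground trace, removes it and subtracts its weight.
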(event Custom|Drop%20Item%20To%20World
  (params (Class :type BP%20Base%20Inventory%20Item%20Class%20Reference) (Spawn%20Transform%20Location :type Vector) (Item%20Info :type S%20Item%20Info%20Structure) (Amount :type Integer))
  (Game|SpawnActorfromClass Class (Math|Transform|MakeTransform Spawn%20Transform%20Location "0, 0, 0" "1,1,1") "Undefined" 0 Item%20Info Amount 0))

(event EventTick
  (params (DeltaSeconds :type Float%20%28single-precision%29)))

(event EventBeginPlay
  (Utilities|Array|Resize (Variables|Default|GetInventory%20Items) (* (Variables|Constant|GetColumn) (Variables|Constant|GetRow))))

(fn Initialization
  (params (Player :type BP%20Base%20Character%20Object%20Reference))
  (Variables|Default|SetPlayer Player))

(fn ToggleInventory
  (bind _ui_inventory_ref (Variables|Default|GetUI%20Inventory%20Ref)
    (:then
      (Widget|RemovefromParent _ui_inventory_ref)
      (Variables|Default|SetUI%20Inventory%20Ref 0)
      (return))
    (:else
      (bind _returnvalue (UserInterface|CreateWidget "/Game/NewInventory/UI/UI_Inventory.UI_Inventory_C" (.AsBP%20My%20Game%20Player%20Controller (Utilities|Casting|CastToBP_MyGamePlayerController (Pawn|GetController (Variables|Default|GetPlayer)))) self (Variables|Default|GetTile%20Size)))
      (Variables|Default|SetUI%20Inventory%20Ref _returnvalue)
      (UserInterface|Viewport|AddtoViewport (Variables|Default|GetUI%20Inventory%20Ref) 0)
      (return))))

(fn InteractItem
  (bind _player (Variables|Default|GetPlayer))
  (bind _interact_actor_array (Variables|/Game/TopDownCPP/Blueprints/BP_Base_Character.BP_Base_Character_C|GetInteract%20Actor%20Array _player))
  (bind _returnvalue (Utilities|Array|LastIndex _interact_actor_array))
  (if (>= _returnvalue 0)
    (Class|BPIInteractItem|Interact(Message) (Utilities|Array|Get(acopy) _interact_actor_array _returnvalue) self)
    (Utilities|Array|Resize _interact_actor_array (Math|Integer|Max(Integer) _returnvalue))
    (return)
    (else
      (return))))

(fn TryAddItem
  (params (Item%20To%20Add :type BP%20Base%20Item%20Object%20Object%20Reference))
  (Utilities|IsValid Item%20To%20Add
    (:Is%20Valid
      (if (> (Default|GetAmount Item%20To%20Add) 0)
        (for (_ _array_index) (Variables|Default|GetInventory%20Items) :!label _label
          (Utilities|CheckItemStacktoAdd _array_index Item%20To%20Add
            (:true
              (Development|PrintString "Stack")
              (return true))
            (:false
              (bind _result (Public|IsSpaceAvailable Item%20To%20Add _array_index))
              (if _result
                (Public|AddItematIndex _array_index Item%20To%20Add)
                (return true)
                (else
                  (Development|PrintString "No Space" true true "(R=0.400714,G=0.000000,B=1.000000,A=1.000000)"))))))
        (Utilities|FlowControl|Sequence
          (:then_0
            (Utilities|FlowControl|DoOnce false
              (:Completed
                (Default|RotateIcon Item%20To%20Add)
                (goto _label))))
          (:then_1
            (Default|RotateIcon Item%20To%20Add)
            (return false)))
        (else
          (Development|PrintString "error amount")
          (return false))))
    (:Is%20Not%20Valid
      (Development|PrintString "Not Valid Item" true true "(R=0.000000,G=1.000000,B=0.199254,A=1.000000)")
      (return false))))

(fn IsSpaceAvailable
  (params (Item%20Object :type BP%20Base%20Item%20Object%20Object%20Reference) (Top%20Left%20Index :type Integer))
  (Utilities|FlowControl|Sequence
    (:then_0
      (bind _tile (Utilities|ForEachIndex Top%20Left%20Index Item%20Object)
        (:LoopBody
          (Utilities|IsTileValid _tile
            (:true
              (bind (_valid _itemobject) (Private|GetItematIndex (Public|TiletoIndex _tile)))
              (if _valid
                (if (Utilities|IsValid _itemobject)
                  (return false))
                (else
                  (return false))))
            (:false
              (return false))))))
    (:then_1
      (return true))))

(fn IndextoTile
  (params (Index :type Integer))
  (bind _column (Variables|Constant|GetColumn))
  (return (Utilities|Struct|MakeS_Inventory_Tile (Math|Integer|%(Integer) Index _column) (/ Index _column))))

(fn GetItematIndex
  (params (Index :type Integer))
  (if (Utilities|Array|IsValidIndex (Variables|Default|GetInventory%20Items) Index)
    (return true (Utilities|Array|Get(acopy) (Variables|Default|GetInventory%20Items) Index))
    (else
      (return false 0))))

(fn TiletoIndex
  (params (Tile :type S%20Inventory%20Tile%20Structure))
  (bind (_x _y) (Utilities|Struct|BreakS_Inventory_Tile Tile))
  (return (+ _x (* _y (Variables|Constant|GetColumn)))))

(fn AddItematIndex
  (params (Top%20Left%20Index :type Integer) (Item%20Object :type BP%20Base%20Item%20Object%20Object%20Reference))
  (bind _tile (Utilities|ForEachIndex Top%20Left%20Index Item%20Object)
    (:LoopBody
      (Utilities|Array|SetArrayElem (Variables|Default|GetInventory%20Items) (Public|TiletoIndex _tile) Item%20Object))
    (:Completed
      (Default|CallOnInventoryChange))))

(fn (Debug)GetItemsList
  (return (Variables|Default|GetInventory%20Items)))

(fn GetAllItems
  (for (_array_element _array_index) (Variables|Default|GetInventory%20Items)
    (bind _output_get (LocalVariables|SetCurrent%20Item%20Object%20Local _array_element))
    (Utilities|IsValid _output_get
      (:Is%20Valid
        (if (not (Utilities|Map|Contains (LocalVariables|GetAll%20Items%20Local) _array_element))
          (Utilities|Map|Add (LocalVariables|GetAll%20Items%20Local) (LocalVariables|GetCurrent%20Item%20Object%20Local) (Public|IndextoTile _array_index))))))
  (return (LocalVariables|GetAll%20Items%20Local)))

(fn RemoveItem
  (params (Item%20Object :type BP%20Base%20Item%20Object%20Object%20Reference))
  (Utilities|IsValid Item%20Object
    (:Is%20Valid
      (for (_array_element _array_index) (Variables|Default|GetInventory%20Items)
        (if (== _array_element Item%20Object)
          (Utilities|Array|SetArrayElem (Variables|Default|GetInventory%20Items) _array_index 0)
          (Default|CallOnInventoryChange))))))

(fn DropItemLocation
  (params (Clamp%20Ground :type Boolean))
  (bind _player (Variables|Default|GetPlayer))
  (LocalVariables|SetSpawn%20Location (+ (Transformation|GetActorLocation _player) (* (Transformation|GetActorForwardVector _player) 1.5e+02)))
  (if Clamp%20Ground
    (bind (_outhit _returnvalue) (Collision|LineTraceByChannel (LocalVariables|GetSpawn%20Location) (- (LocalVariables|GetSpawn%20Location) "0, 0,1000.000000") "TraceTypeQuery1" false (Utilities|Array|MakeArray (Variables|Default|GetPlayer)) "Persistent"))
    (if _returnvalue
      (bind _output_get (LocalVariables|SetSpawn%20Location (.Location (Collision|BreakHitResult _outhit))))
      (return _output_get))))

(fn AddAmount
  (params (Item%20Object :type BP%20Base%20Item%20Object%20Object%20Reference) (Item%20To%20Add :type BP%20Base%20Item%20Object%20Object%20Reference))
  (bind _amount (Default|GetAmount Item%20To%20Add))
  (bind _amount_2 (Default|GetAmount Item%20Object))
  (bind _returnvalue (+ _amount_2 _amount))
  (return _returnvalue (and (not (> _returnvalue (Default|GetMaxAmount Item%20Object))) (== (Default|GetItemClass Item%20Object) (Default|GetItemClass Item%20To%20Add))) _amount))

(fn AddStacktoSlot
  (params (Add%20Item%20To%20Stack :type BP%20Base%20Item%20Object%20Object%20Reference) (Item%20Stack :type BP%20Base%20Item%20Object%20Object%20Reference))
  (bind (_result_amount _add__) (CallFunction|AddAmount Item%20Stack Add%20Item%20To%20Stack))
  (if _add__
    (Default|SetAmount Item%20Stack _result_amount)
    (Default|SetAmount Add%20Item%20To%20Stack)
    (Development|PrintString "set amount stack")
    (return)
    (else
      (Development|PrintString "try add")
      (return))))

(fn SplitStack
  (params (Item%20To%20Split :type BP%20Base%20Item%20Object%20Object%20Reference) (Amount :type Integer))
  (bind _asbp_usable_item_object (Utilities|Casting|CastToBP_Usable_Item_Object Item%20To%20Split))
  (bind _returnvalue (Game|ConstructObjectfromClass "/Game/NewInventory/Blueprint/BP_Usable_Item_Object.BP_Usable_Item_Object_C" self (Default|GetHealthtoAdd _asbp_usable_item_object) (Default|GetItemDimensions Item%20To%20Split) (Default|GetItemIcon Item%20To%20Split) (Default|GetItemClass Item%20To%20Split) (Default|GetItemInfo Item%20To%20Split) (CallFunction|SplitAmount Item%20To%20Split Amount) (Default|GetIsStack? Item%20To%20Split) (Default|GetWeight Item%20To%20Split) (Default|GetMaxAmount Item%20To%20Split) (Default|GetIsUsable Item%20To%20Split) 0))
  (bind _success (Public|TryAddtoSplitStack _returnvalue))
  (if _success
    (return)
    (else
      (bind _success_2 (Public|TryAddItem _returnvalue))
      (if _success_2
        (return)
        (else
          (CallFunction|DropItem _returnvalue)
          (return))))))

(fn SplitAmount
  (params (Item%20To%20Split :type BP%20Base%20Item%20Object%20Object%20Reference) (Amount%20To%20Split :type Integer))
  (Default|SetAmount Item%20To%20Split (- (Default|GetAmount Item%20To%20Split) Amount%20To%20Split))
  (return Amount%20To%20Split))

(fn AddWeight
  (params (Item%20To%20Add :type BP%20Base%20Item%20Object%20Object%20Reference))
  (Variables|Default|SetInventory%20Weight (+ (Variables|Default|GetInventory%20Weight) (* (Default|GetAmount Item%20To%20Add) (Default|GetWeight Item%20To%20Add))))
  (return))

(fn SubtractWeight
  (params (Item%20To%20Remove :type BP%20Base%20Item%20Object%20Object%20Reference))
  (Variables|Default|SetInventory%20Weight (- (Variables|Default|GetInventory%20Weight) (* (Default|GetAmount Item%20To%20Remove) (Default|GetWeight Item%20To%20Remove))))
  (return))

(fn SplitWeight
  (params (Item :type BP%20Base%20Item%20Object%20Object%20Reference) (Amount :type Integer))
  (bind _weight (Default|GetWeight Item))
  (bind _amount (Default|GetAmount Item))
  (bind _returnvalue (+ _amount Amount))
  (bind _returnvalue_2 (Math|Conversions|ToFloat(Integer) _returnvalue))
  (bind _returnvalue_3 (/ _weight _returnvalue_2))
  (bind _returnvalue_4 (* Amount _returnvalue_3))
  (return _returnvalue_4 (- (Default|GetWeight Item) _returnvalue_4)))

(fn DropItem
  (params (Item%20To%20Drop :type BP%20Base%20Item%20Object%20Object%20Reference))
  (CallFunction|DropItemtoWorld (Default|GetItemClass Item%20To%20Drop) (CallFunction|DropItemLocation true) (Default|GetItemInfo Item%20To%20Drop) (Default|GetAmount Item%20To%20Drop))
  (CallFunction|RemoveItem Item%20To%20Drop)
  (CallFunction|SubtractWeight Item%20To%20Drop)
  (return))

(fn ChecktoAutoStack
  (params (Item%20To%20Stack :type BP%20Base%20Item%20Object%20Object%20Reference))
  (Utilities|FlowControl|Sequence
    (:then_0
      (if (Default|GetIsStack? Item%20To%20Stack)
        (for (_ _array_index) (Variables|Default|GetInventory%20Items)
          (bind _tile (Utilities|ForEachIndex _array_index Item%20To%20Stack)
            (:LoopBody
              (Utilities|IsTileValid _tile
                (:true
                  (Utilities|IsValid (Utilities|Array|Get(acopy) (Variables|Default|GetInventory%20Items) (Public|TiletoIndex _tile))
                    (:Is%20Valid
                      (if (.Add%20? (CallFunction|AddAmount (Utilities|Array|Get(acopy) (Variables|Default|GetInventory%20Items) (Public|TiletoIndex _tile)) Item%20To%20Stack))
                        (Default|SetAmount (Utilities|Array|Get(acopy) (Variables|Default|GetInventory%20Items) (Public|TiletoIndex _tile)) (.Result%20Amount (CallFunction|AddAmount (Utilities|Array|Get(acopy) (Variables|Default|GetInventory%20Items) (Public|TiletoIndex _tile)) Item%20To%20Stack)))
                        (Default|SetWeight (Utilities|Array|Get(acopy) (Variables|Default|GetInventory%20Items) (Public|TiletoIndex _tile)) (+ (Default|GetWeight (Utilities|Array|Get(acopy) (Variables|Default|GetInventory%20Items) (Public|TiletoIndex _tile))) (Default|GetWeight Item%20To%20Stack)))
                        (return true)))))))))))
    (:then_1
      (return false))))

(fn TryAddtoSplitStack
  (params (Item%20To%20Add :type BP%20Base%20Item%20Object%20Object%20Reference))
  (Utilities|IsValid Item%20To%20Add
    (:Is%20Valid
      (if (> (Default|GetAmount Item%20To%20Add) 0)
        (for (_ _array_index) (Variables|Default|GetInventory%20Items) :!label _label
          (bind _result (Public|IsSpaceAvailable Item%20To%20Add _array_index))
          (if _result
            (Public|AddItematIndex _array_index Item%20To%20Add)
            (return true)
            (else
              (Development|PrintString "No Space" true true "(R=0.400714,G=0.000000,B=1.000000,A=1.000000)"))))
        (Utilities|FlowControl|Sequence
          (:then_0
            (Utilities|FlowControl|DoOnce false
              (:Completed
                (Default|RotateIcon Item%20To%20Add)
                (goto _label))))
          (:then_1
            (Default|RotateIcon Item%20To%20Add)
            (return false)))
        (else
          (Development|PrintString "error amount")
          (return false))))
    (:Is%20Not%20Valid
      (Development|PrintString "Not Valid Item" true true "(R=0.000000,G=1.000000,B=0.199254,A=1.000000)")
      (return false))))