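; BP_Item_Drag is the drag-and-drop operation for dragging item slots in the inventory system.
; It reaches the inventory's main widget through the dragged slot and toggles that widget's hit testing for the duration of the drag.
; The first drag update makes the widget hit-testable through a DoOnce, and both drop and cancel return it to SelfHitTestInvisible.
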(event EventDragCancelled
  (params (PointerEvent :type Pointer%20Event%20Structure%20%28by%20ref%29))
  (Widget|SetVisibility (Variables|/Game/Inventory_System/Blueprints/BP_Inventory.BP_Inventory_C|GetMain%20Widget (Variables|/Game/Inventory_System/Widget/WB_Inventory_Slot.WB_Inventory_Slot_C|GetInventory%20Ref (Variables|Default|GetDragged%20Slot))) "SelfHitTestInvisible"))

(event EventDragged
  (params (PointerEvent :type Pointer%20Event%20Structure%20%28by%20ref%29))
  (Utilities|FlowControl|DoOnce false
    (:Completed
      (Widget|SetVisibility (Variables|/Game/Inventory_System/Blueprints/BP_Inventory.BP_Inventory_C|GetMain%20Widget (Variables|/Game/Inventory_System/Widget/WB_Inventory_Slot.WB_Inventory_Slot_C|GetInventory%20Ref (Variables|Default|GetDragged%20Slot))) "Visible"))))

(event EventDrop
  (params (PointerEvent :type Pointer%20Event%20Structure%20%28by%20ref%29))
  (Widget|SetVisibility (Variables|/Game/Inventory_System/Blueprints/BP_Inventory.BP_Inventory_C|GetMain%20Widget (Variables|/Game/Inventory_System/Widget/WB_Inventory_Slot.WB_Inventory_Slot_C|GetInventory%20Ref (Variables|Default|GetDragged%20Slot))) "SelfHitTestInvisible"))