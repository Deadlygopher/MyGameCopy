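; Bowl of soup item class for the inventory system, a consumable that heals the character when used.
; On use, it checks the inventory's character reference and, if HP is below max, increases health and removes one unit at its index without spawning it.
; The item actor destroys itself either way, so at full health the inventory entry stays untouched.
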(event EventBeginPlay
  (|CallParentFunction) ; This node is disabled and will not be called.\nDrag off pins to build functionality.
)

(event Collision|EventActorBeginOverlap
  (params (OtherActor :type Actor%20Object%20Reference))
  (|CallParentFunction OtherActor) ; This node is disabled and will not be called.\nDrag off pins to build functionality.
)

(event EventTick
  (params (DeltaSeconds :type Float%20%28single-precision%29))
  (|CallParentFunction DeltaSeconds) ; This node is disabled and will not be called.\nDrag off pins to build functionality.
)

(event EventEventonUsed
  (bind _inventory (Variables|Default|GetInventory))
  (bind _character_ref (Variables|/Game/Inventory_System/Blueprints/BP_Inventory.BP_Inventory_C|GetCharacter%20Ref _inventory))
  (if (< (Variables|/Game/TopDownCPP/Blueprints/BP_Player_Character.BP_Player_Character_C|GetCurent%20HP _character_ref) (Variables|/Game/TopDownCPP/Blueprints/BP_Player_Character.BP_Player_Character_C|GetMax%20HP _character_ref))
    (Default|IncreaseHealth _character_ref 10)
    (Default|RemoveItematIndex (Variables|Default|GetInventory) (Variables|Default|GetIndex) 1 false)
    (Actor|DestroyActor)
    (else
      (Actor|DestroyActor))))

(fn ConstructionScript
  (|CallParentFunction))