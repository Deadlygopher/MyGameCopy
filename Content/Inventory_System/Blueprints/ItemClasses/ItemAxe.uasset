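; Axe item Blueprint for the inventory system that supplies a horizontal attack animation as its first skill and traces the weapon's swing.
; StartTrace calls the parent, then runs a timeline that line-traces from three sphere components to their previous-update positions, covering the swept path between updates.
; The traces use the Visibility channel with persistent debug drawing, and their hit results are not used here.
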(event Custom|SetDefaultTraceLocation
  (Variables|Default|SetTrace_1%20Last%20Location (Transformation|GetWorldLocation (Variables|Default|GetTrace%20Sphere%201)))
  (Variables|Default|SetTrace_2%20Last%20Location (Transformation|GetWorldLocation (Variables|Default|GetTrace%20Sphere%202)))
  (Variables|Default|SetTrace_3%20Last%20Location (Transformation|GetWorldLocation (Variables|Default|GetTrace%20Sphere%203))))

(event EventBeginPlay
  (|CallParentFunction) ; This node is disabled and will not be called.\nDrag off pins to build functionality.
)

(event Collision|EventActorBeginOverlap
  (params (OtherActor :type Actor%20Object%20Reference))
  (|CallParentFunction OtherActor) ; This node is disabled and will not be called.\nDrag off pins to build functionality.
)

(event EventTick
  (params (DeltaSeconds :type Float%20%28single-precision%29))
  (|CallParentFunction DeltaSeconds) ; This node is disabled and will not be called.\nDrag off pins to build functionality.
)

(event EventStartTrace
  (bind _trace_sphere_2 (Variables|Default|GetTrace%20Sphere%202))
  (bind _trace_sphere_3 (Variables|Default|GetTrace%20Sphere%203))
  (bind _trace_sphere_1 (Variables|Default|GetTrace%20Sphere%201))
  (bind _returnvalue (Transformation|GetWorldLocation _trace_sphere_1))
  (bind _returnvalue_2 (Transformation|GetWorldLocation _trace_sphere_2))
  (bind _returnvalue_3 (Transformation|GetWorldLocation _trace_sphere_3))
  (|CallParentFunction)
  (CallFunction|SetDefaultTraceLocation)
  (Timeline|Timeline_0 PlayFromStart
    (:Update
      (Utilities|FlowControl|Sequence
        (:then_0
          (Collision|LineTraceByChannel _returnvalue (Variables|Default|GetTrace_1%20Last%20Location) "TraceTypeQuery1" false 0 "Persistent")
          (Collision|LineTraceByChannel _returnvalue_2 (Variables|Default|GetTrace_2%20Last%20Location) "TraceTypeQuery1" false 0 "Persistent")
          (Collision|LineTraceByChannel _returnvalue_3 (Variables|Default|GetTrace_3%20Last%20Location) "TraceTypeQuery1" false 0 "Persistent"))
        (:then_1
          (Variables|Default|SetTrace_1%20Last%20Location _returnvalue)
          (Variables|Default|SetTrace_2%20Last%20Location _returnvalue_2)
          (Variables|Default|SetTrace_3%20Last%20Location _returnvalue_3))))))

(fn ConstructionScript
  (|CallParentFunction))

(fn FirstSkill
  (bind _output_get (Variables|Default|SetAnimation (Utilities|Struct|MakeSingleAnimationPlayData "/Game/Mannequin/Animations/Character_Anim_Attack_Horizontal.Character_Anim_Attack_Horizontal" false true 0.0)))
  (return _output_get 0.0))