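; World pickup actor for an inventory item, configured from its item class defaults for mesh, scale and interaction radius.
; Sphere overlap registers it in the player's nearby pickup list, showing only the first entry's name/amount widget, or picks up immediately if a pickup command is pending.
; Pickup adds to the inventory, keeping any remainder or destroying the actor.
; Mouse hover swaps material and cursor, showing text when in range.
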(event OnBeginCursorOver(StaticMesh)
  (params (TouchedComponent :type Primitive%20Component%20Object%20Reference))
  (CallFunction|OnHovered))

(event OnComponentBeginOverlap(Sphere)
  (params (OverlappedComponent :type Primitive%20Component%20Object%20Reference) (OtherActor :type Actor%20Object%20Reference) (OtherComp :type Primitive%20Component%20Object%20Reference) (OtherBodyIndex :type Integer) (bFromSweep :type Boolean) (SweepResult :type Hit%20Result%20Structure%20%28by%20ref%29))
  (bind _asbp_player_character (Utilities|Casting|CastToBP_Player_Character OtherActor))
  (Variables|Default|SetIs%20In%20Range%20? true)
  (if (Variables|Default|GetHas%20Pickup%20Command%20?)
    (CallFunction|OnPickup _asbp_player_character)
    (elif (> (Utilities|Array|Length (Variables|/Game/TopDownCPP/Blueprints/BP_Player_Character.BP_Player_Character_C|GetNearby%20Pickup%20Actors _asbp_player_character)) 0)
      (Utilities|Array|Add (Variables|/Game/TopDownCPP/Blueprints/BP_Player_Character.BP_Player_Character_C|GetNearby%20Pickup%20Actors _asbp_player_character) self)
      (else
        (Rendering|SetVisibility (Variables|Default|GetPickup%20Text) true false)
        (Utilities|Array|Add (Variables|/Game/TopDownCPP/Blueprints/BP_Player_Character.BP_Player_Character_C|GetNearby%20Pickup%20Actors _asbp_player_character) self)))))

(event OnComponentEndOverlap(Sphere)
  (params (OverlappedComponent :type Primitive%20Component%20Object%20Reference) (OtherActor :type Actor%20Object%20Reference) (OtherComp :type Primitive%20Component%20Object%20Reference) (OtherBodyIndex :type Integer))
  (bind _asbp_player_character (Utilities|Casting|CastToBP_Player_Character OtherActor))
  (Variables|Default|SetIs%20In%20Range%20? false)
  (if (and (Utilities|IsValid (Utilities|Array|Get(acopy) (Variables|/Game/TopDownCPP/Blueprints/BP_Player_Character.BP_Player_Character_C|GetNearby%20Pickup%20Actors _asbp_player_character))) (== (Utilities|Array|Get(acopy) (Variables|/Game/TopDownCPP/Blueprints/BP_Player_Character.BP_Player_Character_C|GetNearby%20Pickup%20Actors _asbp_player_character)) self))
    (Rendering|SetVisibility (Variables|Default|GetPickup%20Text) false false)
    (Utilities|Array|RemoveItem (Variables|/Game/TopDownCPP/Blueprints/BP_Player_Character.BP_Player_Character_C|GetNearby%20Pickup%20Actors _asbp_player_character) self)
    (Utilities|IsValid (Utilities|Array|Get(acopy) (Variables|/Game/TopDownCPP/Blueprints/BP_Player_Character.BP_Player_Character_C|GetNearby%20Pickup%20Actors _asbp_player_character))
      (:Is%20Valid
        (Rendering|SetVisibility (Variables|BP_PickUp_Actor_C|GetPickup%20Text (Utilities|Array|Get(acopy) (Variables|/Game/TopDownCPP/Blueprints/BP_Player_Character.BP_Player_Character_C|GetNearby%20Pickup%20Actors _asbp_player_character))) true false)))
    (else
      (Utilities|Array|RemoveItem (Variables|/Game/TopDownCPP/Blueprints/BP_Player_Character.BP_Player_Character_C|GetNearby%20Pickup%20Actors _asbp_player_character) self))))

(event OnEndCursorOver(StaticMesh)
  (params (TouchedComponent :type Primitive%20Component%20Object%20Reference))
  (CallFunction|OnUnhovered))

(event Custom|On%20Pickup
  (params (Player%20Character :type BP%20Player%20Character%20Object%20Reference))
  (bind _inventory_ref (Variables|/Game/TopDownCPP/Blueprints/BP_Player_Character.BP_Player_Character_C|GetInventory%20Ref Player%20Character))
  (bind _nearby_pickup_actors (Variables|/Game/TopDownCPP/Blueprints/BP_Player_Character.BP_Player_Character_C|GetNearby%20Pickup%20Actors Player%20Character))
  (bind _output (Utilities|Array|Get(acopy) _nearby_pickup_actors))
  (Utilities|IsValid _inventory_ref
    (:Is%20Valid
      (bind (_success _rest) (Default|AddItem _inventory_ref (Variables|Default|GetItem%20Class) (Variables|Default|GetAmount)))
      (if _success
        (if (> _rest 0)
          (Variables|Default|SetAmount _rest)
          (CallFunction|UpdateText)
          (else
            (Utilities|Array|RemoveItem _nearby_pickup_actors self)
            (Utilities|IsValid _output
              (:Is%20Valid
                (Rendering|SetVisibility (Variables|BP_PickUp_Actor_C|GetPickup%20Text _output) true false))
              (:Is%20Not%20Valid
                _))
            (if (Variables|Default|GetHovered%20?)
              (Variables|/Script/Engine.PlayerController|SetCurrentMouseCursor (Game|GetPlayerController 0) "None")
              (Actor|DestroyActor)
              (else
                (Actor|DestroyActor)))))))))

(event EventBeginPlay
  (CallFunction|UpdateText))

(event Collision|EventActorBeginOverlap
  (params (OtherActor :type Actor%20Object%20Reference)))

(event EventTick
  (params (DeltaSeconds :type Float%20%28single-precision%29)))

(fn ConstructionScript
  (bind _item_class (Variables|Default|GetItem%20Class))
  (bind _static_mesh (Variables|Default|GetStatic%20Mesh))
  (bind _iteminfo (Utilities|GetClassDefaults _item_class))
  (bind (_name _description _icon _canbeused_ _usetext _canbestacked_ _category _pickupmesh _meshscale _interactradius) (Utilities|Struct|BreakS_Item_Info _iteminfo))
  (if (Utilities|IsValidClass _item_class)
    (Components|StaticMesh|SetStaticMesh _static_mesh _pickupmesh)
    (Variables|Default|SetOriginal%20Material (Rendering|Material|GetMaterial _static_mesh 0))
    (Transformation|SetRelativeScale3D (Variables|Default|GetStatic%20Mesh) _meshscale)
    (Components|Sphere|SetSphereRadius (Variables|Default|GetSphere) _interactradius false)))

(fn OnUnhovered
  (Variables|Default|SetHovered%20? false)
  (Variables|/Script/Engine.PlayerController|SetCurrentMouseCursor (Game|GetPlayerController 0) "Default")
  (bind _static_mesh (Variables|Default|GetStatic%20Mesh)
    (:then
      (Rendering|Material|SetMaterial _static_mesh 0 (Variables|Default|GetOriginal%20Material)))
    (:else
      _))
  (return))

(fn UpdateText
  (bind _aswb_pickup_text (Utilities|Casting|CastToWB_Pickup_Text (UserInterface|GetUserWidgetObject (Variables|Default|GetPickup%20Text)))
    (:then
      (Rendering|Components|TextRender|SetText (Variables|/Game/Inventory_System/Widget/WB_Pickup_Text.WB_Pickup_Text_C|GetNameText _aswb_pickup_text) (Utilities|Text|FormatText "{Name} ({Amount})" (.name (.ItemInfo (Utilities|GetClassDefaults (Variables|Default|GetItem%20Class)))) (Variables|Default|GetAmount))))
    (:CastFailed
      _))
  (return))

(fn OnHovered
  (Variables|Default|SetHovered%20? true)
  (Variables|/Script/Engine.PlayerController|SetCurrentMouseCursor (Game|GetPlayerController 0) "Hand")
  (bind _static_mesh (Variables|Default|GetStatic%20Mesh)
    (:then
      (Rendering|Material|SetMaterial _static_mesh 0 "/Game/Inventory_System/Materials/M_Hovered_Pickup.M_Hovered_Pickup"))
    (:else
      _))
  (Rendering|SetVisibility (Variables|Default|GetPickup%20Text) (Variables|Default|GetIs%20In%20Range%20?) false)
  (return))