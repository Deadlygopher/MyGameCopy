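; Equipment component that manages the player's right and left hand weapon slots.
; Adding accepts only BP_Base_Weapon subclasses into an empty slot, sets the player's child actor class, calls its server update and stores the item object.
; Removal clears all three, and SRVSpawnEquipandAttach forwards to the add function.
; Tick prints both slots for debugging, while the socket-based SpawnEquipAndAttach is left unwired in the event graph.
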(event Custom|SRV%20Spawn%20Equip%20and%20Attach
  (params (Item%20Object :type BP%20Base%20Item%20Object%20Object%20Reference) (Selection :type E_Equipment_Type%20Enum :default "NewEnumerator0"))
  (CallFunction|AddItemtoEquipmentSlot Item%20Object Selection))

(event EventTick
  (params (DeltaSeconds :type Float%20%28single-precision%29))
  (Development|PrintString (Utilities|String|Append (Utilities|GetDisplayName (Variables|Default|GetWeapon_Right_Hand)) "///////" (Utilities|GetDisplayName (Variables|Default|GetWeapon_Left_Hand))) true true "(R=0.000000,G=1.000000,B=0.090430,A=1.000000)" 0.0))

(event EventBeginPlay)

(fn RemoveEquip
  (params (Item%20To%20Remove :type BP%20Base%20Item%20Object%20Object%20Reference) (Slot%20Type :type E_Equipment_Type%20Enum :default "NewEnumerator0"))
  (switch Utilities|FlowControl|Switch|SwitchonE_Equipment_Type Slot%20Type
    (:NewEnumerator7
      (Utilities|IsValid (Variables|Default|GetWeapon_Right_Hand)
        (:Is%20Valid
          (ChildActorComponent|SetChildActorClass (Variables|/Game/TopDownCPP/Blueprints/BP_NewInventoryChar.BP_NewInventoryChar_C|GetWeapon%20Right%20Hand (Variables|Default|GetPlayer)) 0)
          (Default|ServerUpdateRightWeaponSlot (Variables|Default|GetPlayer))
          (Variables|Default|SetWeapon_Right_Hand 0)
          (return))))
    (:NewEnumerator8
      (Utilities|IsValid (Variables|Default|GetWeapon_Left_Hand)
        (:Is%20Valid
          (ChildActorComponent|SetChildActorClass (Variables|/Game/TopDownCPP/Blueprints/BP_NewInventoryChar.BP_NewInventoryChar_C|GetWeapon%20Left%20Hand (Variables|Default|GetPlayer)) 0)
          (Default|ServerUpdateLeftWeaponSlot (Variables|Default|GetPlayer))
          (Variables|Default|SetWeapon_Left_Hand 0)
          (return))))))

(fn SpawnEquipandAttach
  (params (Item%20Object :type BP%20Base%20Item%20Object%20Object%20Reference))
  (bind _player (Variables|Default|GetPlayer))
  (bind _returnvalue (Game|SpawnActorfromClass (Default|GetEquipmentClass Item%20Object) (Math|Transform|MakeTransform "0, 0, 0" "0, 0, 0" "1,1,1") "Undefined" _player 0))
  (Transformation|AttachComponentToComponent _returnvalue (Variables|/Script/Engine.Character|GetMesh _player) (Variables|/Game/Equipment/BP_Base_Equipment_Item.BP_Base_Equipment_Item_C|GetSocket%20Name _returnvalue) "SnapToTarget" "SnapToTarget" "SnapToTarget" true)
  (Variables|/Game/Equipment/BP_Base_Equipment_Item.BP_Base_Equipment_Item_C|SetItem%20Object _returnvalue Item%20Object)
  (return _returnvalue))

(fn PlayerInitialization
  (params (Player :type BP%20New%20Inventory%20Char%20Object%20Reference))
  (Variables|Default|SetPlayer Player)
  (return))

(fn AddItemtoEquipmentSlot
  (params (Equip%20Item :type BP%20Base%20Item%20Object%20Object%20Reference) (Selection :type E_Equipment_Type%20Enum :default "NewEnumerator0"))
  (bind _equipment_class (Default|GetEquipmentClass Equip%20Item))
  (bind _equipment_class_2 (Default|GetEquipmentClass Equip%20Item))
  (switch Utilities|FlowControl|Switch|SwitchonE_Equipment_Type Selection
    (:NewEnumerator7
      (if (Utilities|ClassIsChildOf (Default|GetEquipmentClass Equip%20Item) "/Game/Equipment/Weapon/BP_Base_Weapon.BP_Base_Weapon_C")
        (Utilities|IsValid (Variables|Default|GetWeapon_Right_Hand)
          (:Is%20Valid
            (return false))
          (:Is%20Not%20Valid
            (ChildActorComponent|SetChildActorClass (Variables|/Game/TopDownCPP/Blueprints/BP_NewInventoryChar.BP_NewInventoryChar_C|GetWeapon%20Right%20Hand (Variables|Default|GetPlayer)) _equipment_class)
            (Default|ServerUpdateRightWeaponSlot (Variables|Default|GetPlayer) _equipment_class)
            (Variables|Default|SetWeapon_Right_Hand Equip%20Item)
            (return true)))
        (else
          (return false))))
    (:NewEnumerator8
      (if (Utilities|ClassIsChildOf (Default|GetEquipmentClass Equip%20Item) "/Game/Equipment/Weapon/BP_Base_Weapon.BP_Base_Weapon_C")
        (Utilities|IsValid (Variables|Default|GetWeapon_Left_Hand)
          (:Is%20Valid
            (return false))
          (:Is%20Not%20Valid
            (ChildActorComponent|SetChildActorClass (Variables|/Game/TopDownCPP/Blueprints/BP_NewInventoryChar.BP_NewInventoryChar_C|GetWeapon%20Left%20Hand (Variables|Default|GetPlayer)) _equipment_class_2)
            (Default|ServerUpdateLeftWeaponSlot (Variables|Default|GetPlayer) _equipment_class_2)
            (Variables|Default|SetWeapon_Left_Hand Equip%20Item)
            (return true)))
        (else
          (return false))))))