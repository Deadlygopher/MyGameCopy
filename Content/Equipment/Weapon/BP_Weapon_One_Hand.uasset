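; One-handed weapon Blueprint that detects melee hits on pawns during a swing and supplies a first-skill animation montage with its duration.
; BeginTrace runs a timeline that line-traces each update from three blade spheres back to their last positions, covering the swept path between frames.
; The first pawn hit blocks further traces and, if it is a BP_NewInventoryChar, receives WeaponDamageMessage with Damage.
; EndTrace stops the timeline.
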(event EventBeginPlay
  (|CallParentFunction) ; This node is disabled and will not be called.\nDrag off pins to build functionality.
)

(event Collision|EventActorBeginOverlap
  (params (OtherActor :type Actor%20Object%20Reference))
  (|CallParentFunction OtherActor) ; This node is disabled and will not be called.\nDrag off pins to build functionality.
)

(event EventTick
  (params (DeltaSeconds :type Float%20%28single-precision%29))
  (|CallParentFunction DeltaSeconds) ; This node is disabled and will not be called.\nDrag off pins to build functionality.
)

(event EventEndTrace
  (bind _array (Utilities|Array|MakeArray "ObjectTypeQuery3"))
  (bind _trace_sphere_1 (Variables|Default|GetTrace%20Sphere%201))
  (bind _trace_sphere_2 (Variables|Default|GetTrace%20Sphere%202))
  (bind _trace_sphere_3 (Variables|Default|GetTrace%20Sphere%203))
  (bind _returnvalue (Transformation|GetWorldLocation _trace_sphere_1))
  (bind _returnvalue_2 (Transformation|GetWorldLocation _trace_sphere_2))
  (bind _returnvalue_3 (Transformation|GetWorldLocation _trace_sphere_3))
  (Timeline|Timeline Stop
    (:Update
      (if (not (Variables|Default|GetBlocking%20Hit))
        (Utilities|FlowControl|Sequence
          (:then_0
            (bind (_outhit _returnvalue_4) (Collision|LineTraceForObjects _returnvalue (Variables|Default|GetTrace%201%20Last%20Location) _array false (Utilities|Array|MakeArray (stale EventBeginTrace Ignore%20Actor)) "ForDuration"))
            (if _returnvalue_4
              (bind _output_get (Variables|Default|SetHit%20Actor (.HitActor (Collision|BreakHitResult _outhit))))
              (Variables|Default|SetBlocking%20Hit (Utilities|ClassIsChildOf (Utilities|GetClass _output_get) "/Script/Engine.Pawn"))
              (bind _asbp_new_inventory_char (Utilities|Casting|CastToBP_NewInventoryChar _output_get))
              (Class|BPIWeaponDamage|WeaponDamage(Message) _asbp_new_inventory_char (Variables|Default|GetDamage))
              (else
                (bind (_outhit_2 _returnvalue_5) (Collision|LineTraceForObjects _returnvalue_2 (Variables|Default|GetTrace%202%20Last%20Location) _array false (Utilities|Array|MakeArray (stale EventBeginTrace Ignore%20Actor)) "ForDuration"))
                (if _returnvalue_5
                  (bind _output_get_2 (Variables|Default|SetHit%20Actor (.HitActor (Collision|BreakHitResult _outhit_2))))
                  (Variables|Default|SetBlocking%20Hit (Utilities|ClassIsChildOf (Utilities|GetClass _output_get_2) "/Script/Engine.Pawn"))
                  (bind _asbp_new_inventory_char_2 (Utilities|Casting|CastToBP_NewInventoryChar _output_get_2))
                  (Class|BPIWeaponDamage|WeaponDamage(Message) _asbp_new_inventory_char_2 (Variables|Default|GetDamage))
                  (else
                    (bind (_outhit_3 _returnvalue_6) (Collision|LineTraceForObjects _returnvalue_3 (Variables|Default|GetTrace%203%20Last%20Location) _array false (Utilities|Array|MakeArray (stale EventBeginTrace Ignore%20Actor)) "ForDuration"))
                    (if _returnvalue_6
                      (bind _output_get_3 (Variables|Default|SetHit%20Actor (.HitActor (Collision|BreakHitResult _outhit_3))))
                      (Variables|Default|SetBlocking%20Hit (Utilities|ClassIsChildOf (Utilities|GetClass _output_get_3) "/Script/Engine.Pawn"))
                      (bind _asbp_new_inventory_char_3 (Utilities|Casting|CastToBP_NewInventoryChar _output_get_3))
                      (Class|BPIWeaponDamage|WeaponDamage(Message) _asbp_new_inventory_char_3 (Variables|Default|GetDamage))))))))
          (:then_1
            (Variables|Default|SetTrace%201%20Last%20Location _returnvalue)
            (Variables|Default|SetTrace%202%20Last%20Location _returnvalue_2)
            (Variables|Default|SetTrace%203%20Last%20Location _returnvalue_3)))))))

(event EventBeginTrace
  (params (Ignore%20Actor :type Actor%20Object%20Reference))
  (bind _array (Utilities|Array|MakeArray Ignore%20Actor))
  (bind _array_2 (Utilities|Array|MakeArray "ObjectTypeQuery3"))
  (bind _trace_sphere_1 (Variables|Default|GetTrace%20Sphere%201))
  (bind _trace_sphere_2 (Variables|Default|GetTrace%20Sphere%202))
  (bind _trace_sphere_3 (Variables|Default|GetTrace%20Sphere%203))
  (bind _returnvalue (Transformation|GetWorldLocation _trace_sphere_1))
  (bind _returnvalue_2 (Transformation|GetWorldLocation _trace_sphere_2))
  (bind _returnvalue_3 (Transformation|GetWorldLocation _trace_sphere_3))
  (Variables|Default|SetBlocking%20Hit false)
  (CallFunction|ResetTraceLocations)
  (Timeline|Timeline PlayFromStart
    (:Update
      (if (not (Variables|Default|GetBlocking%20Hit))
        (Utilities|FlowControl|Sequence
          (:then_0
            (bind (_outhit _returnvalue_4) (Collision|LineTraceForObjects _returnvalue (Variables|Default|GetTrace%201%20Last%20Location) _array_2 false _array "ForDuration"))
            (if _returnvalue_4
              (bind _output_get (Variables|Default|SetHit%20Actor (.HitActor (Collision|BreakHitResult _outhit))))
              (Variables|Default|SetBlocking%20Hit (Utilities|ClassIsChildOf (Utilities|GetClass _output_get) "/Script/Engine.Pawn"))
              (bind _asbp_new_inventory_char (Utilities|Casting|CastToBP_NewInventoryChar _output_get))
              (Class|BPIWeaponDamage|WeaponDamage(Message) _asbp_new_inventory_char (Variables|Default|GetDamage))
              (else
                (bind (_outhit_2 _returnvalue_5) (Collision|LineTraceForObjects _returnvalue_2 (Variables|Default|GetTrace%202%20Last%20Location) _array_2 false _array "ForDuration"))
                (if _returnvalue_5
                  (bind _output_get_2 (Variables|Default|SetHit%20Actor (.HitActor (Collision|BreakHitResult _outhit_2))))
                  (Variables|Default|SetBlocking%20Hit (Utilities|ClassIsChildOf (Utilities|GetClass _output_get_2) "/Script/Engine.Pawn"))
                  (bind _asbp_new_inventory_char_2 (Utilities|Casting|CastToBP_NewInventoryChar _output_get_2))
                  (Class|BPIWeaponDamage|WeaponDamage(Message) _asbp_new_inventory_char_2 (Variables|Default|GetDamage))
                  (else
                    (bind (_outhit_3 _returnvalue_6) (Collision|LineTraceForObjects _returnvalue_3 (Variables|Default|GetTrace%203%20Last%20Location) _array_2 false _array "ForDuration"))
                    (if _returnvalue_6
                      (bind _output_get_3 (Variables|Default|SetHit%20Actor (.HitActor (Collision|BreakHitResult _outhit_3))))
                      (Variables|Default|SetBlocking%20Hit (Utilities|ClassIsChildOf (Utilities|GetClass _output_get_3) "/Script/Engine.Pawn"))
                      (bind _asbp_new_inventory_char_3 (Utilities|Casting|CastToBP_NewInventoryChar _output_get_3))
                      (Class|BPIWeaponDamage|WeaponDamage(Message) _asbp_new_inventory_char_3 (Variables|Default|GetDamage))))))))
          (:then_1
            (Variables|Default|SetTrace%201%20Last%20Location _returnvalue)
            (Variables|Default|SetTrace%202%20Last%20Location _returnvalue_2)
            (Variables|Default|SetTrace%203%20Last%20Location _returnvalue_3)))))))

(fn ConstructionScript
  (|CallParentFunction))

(fn ResetTraceLocations
  (Variables|Default|SetTrace%201%20Last%20Location (Transformation|GetWorldLocation (Variables|Default|GetTrace%20Sphere%201)))
  (Variables|Default|SetTrace%202%20Last%20Location (Transformation|GetWorldLocation (Variables|Default|GetTrace%20Sphere%202)))
  (Variables|Default|SetTrace%203%20Last%20Location (Transformation|GetWorldLocation (Variables|Default|GetTrace%20Sphere%203))))

(fn FirstSkill
  (return (Variables|Default|GetFirst%20Skill%20Animation%20Montage) (Variables|Default|GetFirst%20Skill%20Animation%20Duration)))