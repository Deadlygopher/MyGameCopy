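; Simple bow weapon Blueprint that animates drawing and firing and measures how long each shot was aimed.
; EventAim plays the pull animation, stores the start time and flags the bow as aiming.
; EventShot acts only while aiming: it plays the fire animation, computes and prints the elapsed aim time, then clears the flag.
; GetTotalAimingTime exposes that duration; no projectile or damage logic is present here.
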(event EventBeginPlay
  (|CallParentFunction) ; This node is disabled and will not be called.\nDrag off pins to build functionality.
)

(event Collision|EventActorBeginOverlap
  (params (OtherActor :type Actor%20Object%20Reference))
  (|CallParentFunction OtherActor))

(event EventTick
  (params (DeltaSeconds :type Float%20%28single-precision%29))
  (|CallParentFunction DeltaSeconds))

(event EventEventAim
  (Components|Animation|PlayAnimation (Variables|Default|GetSkeletalMesh) "/Game/HB_MedievalWeapPack3/Animation/HB_SM_Bow_PULL.HB_SM_Bow_PULL" false)
  (Variables|Default|SetAim%20Start%20Time 0.0)
  (Variables|Default|SetAim%20Start%20Time (Utilities|Time|GetTimeSeconds))
  (Variables|Default|SetAiming%20? true))

(event EventEventShot
  (if (Variables|Default|GetAiming%20?)
    (Components|Animation|PlayAnimation (Variables|Default|GetSkeletalMesh) "/Game/HB_MedievalWeapPack3/Animation/HB_SM_Bow_FIRE.HB_SM_Bow_FIRE" false)
    (Variables|Default|SetAim%20End%20Time 0.0)
    (bind _output_get (Variables|Default|SetAim%20End%20Time (Utilities|Time|GetTimeSeconds)))
    (bind _output_get_2 (Variables|Default|SetTotal%20Aim%20Time (- _output_get (Variables|Default|GetAim%20Start%20Time))))
    (Variables|Default|SetAiming%20? false)
    (Development|PrintString (Utilities|String|ToString(Float) _output_get_2))))

(fn ConstructionScript
  (|CallParentFunction))

(fn GetTotalAimingTime
  (return (Variables|Default|GetTotal%20Aim%20Time)))