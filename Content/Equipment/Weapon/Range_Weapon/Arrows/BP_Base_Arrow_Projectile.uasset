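; Base arrow projectile for ranged weapons that damages characters and sticks into whatever it hits.
; The construction script feeds InitialSpeed into the projectile movement component.
; On capsule overlap it stops movement and gravity, sends characters damage scaled from InitialSpeed, attaches to their mesh socket or the other actor, then disables collision.
; GetTotalAimingTime is a stub returning zero.
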(event OnComponentBeginOverlap(Capsule)
  (params (OverlappedComponent :type Primitive%20Component%20Object%20Reference) (OtherActor :type Actor%20Object%20Reference) (OtherComp :type Primitive%20Component%20Object%20Reference) (OtherBodyIndex :type Integer) (bFromSweep :type Boolean) (SweepResult :type Hit%20Result%20Structure%20%28by%20ref%29))
  (bind _projectilemovement (Variables|Default|GetProjectileMovement))
  (if (!= OtherActor self)
    (Components|Movement|StopMovementImmediately _projectilemovement)
    (Variables|/Script/Engine.ProjectileMovementComponent|SetProjectileGravityScale _projectilemovement 0.0)
    (bind _asbp_base_character (Utilities|Casting|CastToBP_Base_Character OtherActor)
      (:then
        (Class|BPIWeaponDamage|WeaponDamage(Message) _asbp_base_character (/ (Variables|Default|GetInitial%20Speed) 1e+02))
        (Transformation|AttachComponentToComponent (Variables|/Script/Engine.Character|GetMesh _asbp_base_character) "Arrow_Attach_Socket" "KeepWorld" "KeepWorld" "KeepWorld" true)
        (Collision|SetCollisionEnabled (Variables|Default|GetCapsule) "NoCollision"))
      (:CastFailed
        (Transformation|AttachActorToActor OtherActor "None" "KeepWorld" "KeepWorld" "KeepWorld" true)
        (Collision|SetCollisionEnabled (Variables|Default|GetCapsule) "NoCollision")))))

(event EventBeginPlay)

(event Collision|EventActorBeginOverlap
  (params (OtherActor :type Actor%20Object%20Reference)))

(event EventTick
  (params (DeltaSeconds :type Float%20%28single-precision%29)))

(fn ConstructionScript
  (Variables|/Script/Engine.ProjectileMovementComponent|SetInitialSpeed (Variables|Default|GetProjectileMovement) (Variables|Default|GetInitial%20Speed)))

(fn GetTotalAimingTime
  (return 0.0))