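; AI controller for BP_NewInventoryChar enemies that hunt and attack other characters of that class with melee weapons.
; On BeginPlay it randomly picks axe or mace for the right hand and runs a behavior tree.
; Perception updates from living characters set the blackboard's Player key, or clear it and store Last Seen Location when lost.
; Helper functions play the weapon attack via a server animation call and check whether the detected pawn is dead.
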(event OnTargetPerceptionUpdated(AIPerception)
  (params (Actor :type Actor%20Object%20Reference) (Stimulus :type AI%20Stimulus%20Structure))
  (bind _asbp_new_inventory_char (Utilities|Casting|CastToBP_NewInventoryChar Actor))
  (if (not (<= (Variables|/Game/TopDownCPP/Blueprints/BPC_Player_State.BPC_Player_State_C|GetHealth (Variables|/Game/TopDownCPP/Blueprints/BP_NewInventoryChar.BP_NewInventoryChar_C|GetBPC_Player_State _asbp_new_inventory_char)) 0.0))
    (if (.bsuccessfullysensed Stimulus)
      (bind _output_get (Variables|Default|SetDetected%20Pawn Actor))
      (AI|Components|Blackboard|SetValueasObject (Variables|Default|GetAI_Blackboard) (Utilities|String|StringToName "Player") _output_get)
      (else
        (Variables|Default|SetDetected%20Pawn 0)
        (AI|Components|Blackboard|ClearValue (Variables|Default|GetAI_Blackboard) (Utilities|String|StringToName "Player"))
        (AI|Components|Blackboard|SetValueasVector (Variables|Default|GetAI_Blackboard) (Utilities|String|StringToName "Last Seen Location") (.stimuluslocation Stimulus))))))

(event EventBeginPlay
  (bind _returnvalue (Math|Random|RandomIntegerinRange 0 1))
  (bind _returnvalue_2 (Utilities|Select :Index _returnvalue :Option%200 "/Game/Equipment/Weapon/BP_Axe_Weapon.BP_Axe_Weapon_C" :Option%201 "/Game/Equipment/Weapon/BP_Mace_Weapon.BP_Mace_Weapon_C"))
  (bind _asbp_new_inventory_char (Utilities|Casting|CastToBP_NewInventoryChar (Pawn|GetControlledPawn)))
  (bind _output_get (Variables|Default|SetControlled%20Pawn _asbp_new_inventory_char))
  (ChildActorComponent|SetChildActorClass (Variables|/Game/TopDownCPP/Blueprints/BP_NewInventoryChar.BP_NewInventoryChar_C|GetWeapon%20Right%20Hand _output_get) _returnvalue_2)
  (Default|ServerUpdateRightWeaponSlot (Variables|Default|GetControlled%20Pawn) _returnvalue_2)
  (AI|RunBehaviorTree (Variables|Default|GetBehavior%20Tree)))

(event EventTick
  (params (DeltaSeconds :type Float%20%28single-precision%29)))

(fn ConstructionScript)

(fn AIAttack
  (bind _controlled_pawn (Variables|Default|GetControlled%20Pawn))
  (bind _weapon_right_hand (Variables|/Game/TopDownCPP/Blueprints/BP_NewInventoryChar.BP_NewInventoryChar_C|GetWeapon%20Right%20Hand _controlled_pawn))
  (Utilities|IsValid _weapon_right_hand
    (:Is%20Valid
      (Default|ServerPlayAnimation _controlled_pawn (Variables|/Script/Engine.ChildActorComponent|GetChildActor _weapon_right_hand))
      (return))
    (:Is%20Not%20Valid
      (return))))

(fn IsPawnDeath?
  (params (InputObject :type Object%20Object%20Reference))
  (Utilities|IsValid InputObject
    (:Is%20Valid
      (bind _asbp_new_inventory_char (Utilities|Casting|CastToBP_NewInventoryChar (Variables|Default|GetDetected%20Pawn)))
      (if (<= (Variables|/Game/TopDownCPP/Blueprints/BPC_Player_State.BPC_Player_State_C|GetHealth (Variables|/Game/TopDownCPP/Blueprints/BP_NewInventoryChar.BP_NewInventoryChar_C|GetBPC_Player_State _asbp_new_inventory_char)) 0.0)
        (return true)
        (else
          (return false))))))